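; Two-player Pong game logic that simulates the ball and paddles in normalized 0–1 space and renders through the MP_Pong material parameter collection.
; Tick moves the ball by a fixed per-frame step, bounces it off top, bottom and paddles, and on side exits scores, resets and updates score texts.
; W/S and arrow keys step each paddle per press, pushing new positions to the collection.
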(event `self.ReceiveBeginPlay`
  (bind (_x _y) (`KismetMathLibrary.BreakVector2D` (`self.PaddleDimension`)))
  (`KismetMaterialLibrary.SetScalarParameterValue` "/Game/Pong/MP_Pong.MP_Pong" "u_ballRadius" (`self.BallRadius`))
  (`KismetMaterialLibrary.SetScalarParameterValue` "/Game/Pong/MP_Pong.MP_Pong" "u_Paddle1Y" (`self.Paddle1Y`))
  (`KismetMaterialLibrary.SetScalarParameterValue` "/Game/Pong/MP_Pong.MP_Pong" "u_Paddle2Y" (`self.Paddle2Y`))
  (`KismetMaterialLibrary.SetScalarParameterValue` "/Game/Pong/MP_Pong.MP_Pong" "u_PaddleWidth" _x)
  (`KismetMaterialLibrary.SetScalarParameterValue` "/Game/Pong/MP_Pong.MP_Pong" "u_PaddleHeight" _y)
  (`KismetMaterialLibrary.SetScalarParameterValue` "/Game/Pong/MP_Pong.MP_Pong" "u_Paddle1X" (`self.Paddle1X`))
  (`KismetMaterialLibrary.SetScalarParameterValue` "/Game/Pong/MP_Pong.MP_Pong" "u_Paddle2X" (`self.Paddle2X`)))

(event `self.ReceiveTick`
  (params (DeltaSeconds :type "Float (single-precision)"))
  (bind _ballradius (`self.BallRadius`))
  (bind _paddle2y (`self.Paddle2Y`))
  (bind _paddle1y (`self.Paddle1Y`))
  (bind _ballradius_2 (`self.BallRadius`))
  (bind _ballradius_3 (`self.BallRadius`))
  (bind _x (`KismetMathLibrary.BreakVector2D` (`self.BallPos`)))
  (bind (_x_2 _y) (`KismetMathLibrary.BreakVector2D` (`self.BallVel`)))
  (bind (_x_3 _y_2) (`KismetMathLibrary.BreakVector2D` (`self.BallPos`)))
  (bind (_x_4 _y_3) (`KismetMathLibrary.BreakVector2D` (`self.PaddleDimension`)))
  (bind (_x_5 _y_4) (`KismetMathLibrary.BreakVector2D` (`self.BallPos`)))
  (bind (_x_6 _y_5) (`KismetMathLibrary.BreakVector2D` (`self.BallVel`)))
  (bind (_x_7 _y_6) (`KismetMathLibrary.BreakVector2D` (`self.PaddleDimension`)))
  (bind (_x_8 _y_7) (`KismetMathLibrary.BreakVector2D` (`self.BallPos`)))
  (bind (_x_9 _y_8) (`KismetMathLibrary.BreakVector2D` (`self.BallVel`)))
  (set `self.Delta Seconds` DeltaSeconds)
  (set `self.BallPos` (+ (`self.BallPos`) (`self.BallVel`)))
  (`|ExecutionSequence`
    (:`then_0`
      (if (>= (+ _x _ballradius_2) 1.0)
        (`/Engine/EditorBlueprintResources/StandardMacros.IncrementInt` (`self.Paddle1Score`)
          (:`  `
            (set `self.BallPos` (0.5 0.5) :!label _label)
            (set `self.BallVel` (0.0075 -0.00375))
            (`TextRenderComponent.K2_SetText` (`self.Paddle2Sc`) (`KismetTextLibrary.Conv_IntToText` (`self.Paddle1Score`)))
            (`TextRenderComponent.K2_SetText` (`self.Paddle1Sc`) (`KismetTextLibrary.Conv_IntToText` (`self.Paddle2Score`)))))
        (elif (<= (- _x _ballradius_2) 0.0)
          (`/Engine/EditorBlueprintResources/StandardMacros.IncrementInt` (`self.Paddle2Score`)
            (:`  `
              (goto _label))))))
    (:`then_1`
      (if (`self.IsBallYInRange` 0.0 1.0)
        (set `self.BallVel` (`KismetMathLibrary.MakeVector2D` _x_9 (* _y_8 -1.0)))))
    (:`then_2`
      (if (and (<= (- (`KismetMathLibrary.BreakVector2D` (`self.BallPos`)) (`self.BallRadius`)) (+ (`self.Paddle1X`) (/ (`KismetMathLibrary.BreakVector2D` (`self.PaddleDimension`)) 2.0))) (and (<= (+ _y_4 _ballradius_3) (+ _paddle1y _y_3)) (>= (- _y_4 _ballradius_3) (- _paddle1y _y_3))))
        (set `self.BallVel` (`KismetMathLibrary.MakeVector2D` (* _x_2 -1.0) _y))))
    (:`then_3`
      (if (and (>= (+ (`KismetMathLibrary.BreakVector2D` (`self.BallPos`)) (`self.BallRadius`)) (- (`self.Paddle2X`) (/ (`KismetMathLibrary.BreakVector2D` (`self.PaddleDimension`)) 2.0))) (and (<= (+ _y_7 _ballradius) (+ _paddle2y _y_6)) (>= (- _y_7 _ballradius) (- _paddle2y _y_6))))
        (set `self.BallVel` (`KismetMathLibrary.MakeVector2D` (* _x_6 -1.0) _y_5))))
    (:`then_4`
      (`KismetMaterialLibrary.SetScalarParameterValue` "/Game/Pong/MP_Pong.MP_Pong" "u_ballPosX" _x_3)
      (`KismetMaterialLibrary.SetScalarParameterValue` "/Game/Pong/MP_Pong.MP_Pong" "u_ballPosY" _y_2))))

(event `InputAction|W_Up` :consume false
  (params (Key :type "Key Structure"))
  (:`Pressed`
    (`KismetSystemLibrary.PrintText` (`KismetInputLibrary.Key_GetDisplayName` Key))
    (set `self.Paddle1Y` (- (`self.Paddle1Y`) (`self.PaddleVelocity`)))
    (`KismetMaterialLibrary.SetScalarParameterValue` "/Game/Pong/MP_Pong.MP_Pong" "u_Paddle1Y" (`self.Paddle1Y`) :!label _label_2)))

(event `InputAction|S_Down` :consume false
  (params (Key :type "Key Structure"))
  (:`Pressed`
    (`KismetSystemLibrary.PrintText` (`KismetInputLibrary.Key_GetDisplayName` Key))
    (set `self.Paddle1Y` (+ (`self.Paddle1Y`) (`self.PaddleVelocity`)))
    (goto _label_2)))

(event `InputAction|ArrowUp` :consume false
  (params (Key :type "Key Structure"))
  (:`Pressed`
    (`KismetSystemLibrary.PrintText` (`KismetInputLibrary.Key_GetDisplayName` Key))
    (set `self.Paddle2Y` (- (`self.Paddle2Y`) (`self.PaddleVelocity`)))
    (`KismetMaterialLibrary.SetScalarParameterValue` "/Game/Pong/MP_Pong.MP_Pong" "u_Paddle2Y" (`self.Paddle2Y`) :!label _label_3)))

(event `InputAction|ArrowDown` :consume false
  (params (Key :type "Key Structure"))
  (:`Pressed`
    (`KismetSystemLibrary.PrintText` (`KismetInputLibrary.Key_GetDisplayName` Key))
    (set `self.Paddle2Y` (+ (`self.Paddle2Y`) (`self.PaddleVelocity`)))
    (goto _label_3)))

(fn `UserConstructionScript`
  (`KismetMaterialLibrary.SetScalarParameterValue` "/Game/Pong/MP_Pong.MP_Pong" "u_ballRadius" (`self.BallRadius`))
  (`KismetMaterialLibrary.SetScalarParameterValue` "/Game/Pong/MP_Pong.MP_Pong" "u_Paddle1Y" (`self.Paddle1Y`))
  (`KismetMaterialLibrary.SetScalarParameterValue` "/Game/Pong/MP_Pong.MP_Pong" "u_Paddle2Y" (`self.Paddle2Y`)))