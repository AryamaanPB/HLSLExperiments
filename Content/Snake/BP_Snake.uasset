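; Snake game controller that moves a snake by writing its position and size to the MP_Snake Material Parameter Collection, presumably for a material to draw.
; Tick accumulates time and, at each interval, steps the position along the current axis by velocity times speed.
; WASD input allows only perpendicular turns, and each turn also randomizes the RandCube position parameters.
; No growth, collision or bounds logic exists; several position-nudge chains are unconnected leftovers.
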(event `self.ReceiveBeginPlay`
  (`KismetMaterialLibrary.SetScalarParameterValue` "/Game/Snake/MP_Snake.MP_Snake" "SnakeDim" (`self.SnakeDim`)))

(event `self.ReceiveTick`
  (params (DeltaSeconds :type "Float (single-precision)"))
  (bind _returnvalue (* (`self.SnakeVel`) (`self.SnakeSpeed`)))
  (bind _output_get (set `self.TimeSinceLastMove` (+ DeltaSeconds (`self.TimeSinceLastMove`))))
  (if (>= _output_get (`self.TimeInterval`))
    (set `self.TimeSinceLastMove` 0.0)
    (if (`self.SnakeDir`)
      (bind _output_get_2 (set `self.SnakePosY` (+ _returnvalue (`self.SnakePosY`))))
      (`KismetMaterialLibrary.SetScalarParameterValue` "/Game/Snake/MP_Snake.MP_Snake" "SnakePosY" _output_get_2)
      (else
        (bind _output_get_3 (set `self.SnakePosX` (+ _returnvalue (`self.SnakePosX`))))
        (`KismetMaterialLibrary.SetScalarParameterValue` "/Game/Snake/MP_Snake.MP_Snake" "SnakePosX" _output_get_3)))))

(event `InputAction|A_Left`
  (params (Key :type "Key Structure"))
  (:`Pressed`
    (if (`self.SnakeDir`)
      (set `self.SnakeDir` false)
      (set `self.SnakeVel` -1)
      (`KismetMaterialLibrary.SetScalarParameterValue` "/Game/Snake/MP_Snake.MP_Snake" "RandCubePosX" (`KismetMathLibrary.RandomFloatInRange` 0.0 1.0) :!label _label)
      (`KismetMaterialLibrary.SetScalarParameterValue` "/Game/Snake/MP_Snake.MP_Snake" "RandCubePosY" (`KismetMathLibrary.RandomFloatInRange` 0.0 1.0)))))

(event `InputAction|D_Right`
  (params (Key :type "Key Structure"))
  (:`Pressed`
    (if (`self.SnakeDir`)
      (set `self.SnakeDir` false)
      (set `self.SnakeVel` 1)
      (goto _label))))

(event `InputAction|W_Up`
  (params (Key :type "Key Structure"))
  (:`Pressed`
    (if (not (`self.SnakeDir`))
      (set `self.SnakeDir` true)
      (set `self.SnakeVel` -1)
      (goto _label))))

(event `InputAction|S_Down`
  (params (Key :type "Key Structure"))
  (:`Pressed`
    (if (not (`self.SnakeDir`))
      (set `self.SnakeDir` true)
      (set `self.SnakeVel` 1)
      (goto _label))))

(fn `UserConstructionScript`)