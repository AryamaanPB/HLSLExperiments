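; Pong game Blueprint that simulates ball and paddles in 2D and passes their state to the MP_Pong material parameter collection, presumably for shader drawing.
; Tick advances the ball per frame without delta scaling, flipping velocity on range checks and on Paddle1's X edge, ignoring paddle height and Paddle2.
; Input presses step each paddle's Y and update the collection.
; BeginPlay blocks player look and move input and seeds the parameters.
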(event `self.ReceiveBeginPlay`
  (bind _returnvalue (`GameplayStatics.GetPlayerController` 0))
  (bind (_x _y) (`KismetMathLibrary.BreakVector2D` (`self.PaddleDimension`)))
  (`Controller.SetIgnoreLookInput` _returnvalue true)
  (`Controller.SetIgnoreMoveInput` _returnvalue true)
  (`KismetMaterialLibrary.SetScalarParameterValue` "/Game/MP_Pong.MP_Pong" "u_ballRadius" (`self.BallRadius`))
  (`KismetMaterialLibrary.SetScalarParameterValue` "/Game/MP_Pong.MP_Pong" "u_Paddle1Y" (`self.Paddle1Y`))
  (`KismetMaterialLibrary.SetScalarParameterValue` "/Game/MP_Pong.MP_Pong" "u_Paddle2Y" (`self.Paddle2Y`))
  (`KismetMaterialLibrary.SetScalarParameterValue` "/Game/MP_Pong.MP_Pong" "u_PaddleWidth" _x)
  (`KismetMaterialLibrary.SetScalarParameterValue` "/Game/MP_Pong.MP_Pong" "u_PaddleHeight" _y)
  (`KismetMaterialLibrary.SetScalarParameterValue` "/Game/MP_Pong.MP_Pong" "u_Paddle1X" (`self.Paddle1X`))
  (`KismetMaterialLibrary.SetScalarParameterValue` "/Game/MP_Pong.MP_Pong" "u_Paddle2X" (`self.Paddle2X`)))

(event `self.ReceiveTick`
  (params (DeltaSeconds :type "Float (single-precision)"))
  (bind (_x _y) (`KismetMathLibrary.BreakVector2D` (`self.BallVel`)))
  (bind (_x_2 _y_2) (`KismetMathLibrary.BreakVector2D` (`self.BallPos`)))
  (bind (_x_3 _y_3) (`KismetMathLibrary.BreakVector2D` (`self.BallVel`)))
  (bind (_x_4 _y_4) (`KismetMathLibrary.BreakVector2D` (`self.BallVel`)))
  (set `self.Delta Seconds` DeltaSeconds)
  (set `self.BallPos` (+ (`self.BallPos`) (`self.BallVel`)))
  (`|ExecutionSequence`
    (:`then_0`
      (if (`self.IsBallXInRange` 0.0)
        (set `self.BallVel` (`KismetMathLibrary.MakeVector2D` (* _x_3 -1.0) _y_3))))
    (:`then_1`
      (if (`self.IsBallYInRange` 0.0 1.0)
        (set `self.BallVel` (`KismetMathLibrary.MakeVector2D` _x_4 (* _y_4 -1.0)))))
    (:`then_2`
      (if (<= (- (`KismetMathLibrary.BreakVector2D` (`self.BallPos`)) (`self.BallRadius`)) (+ (`self.Paddle1X`) (`KismetMathLibrary.BreakVector2D` (`self.PaddleDimension`))))
        (set `self.BallVel` (`KismetMathLibrary.MakeVector2D` (* _x -1.0) _y))))
    (:`then_4`
      (`KismetMaterialLibrary.SetScalarParameterValue` "/Game/MP_Pong.MP_Pong" "u_ballPosX" _x_2)
      (`KismetMaterialLibrary.SetScalarParameterValue` "/Game/MP_Pong.MP_Pong" "u_ballPosY" _y_2))))

(event `InputAction|Paddle1Up`
  (params (Key :type "Key Structure"))
  (:`Pressed`
    (set `self.Paddle1Y` (- (`self.Paddle1Y`) (`self.PaddleVelocity`)))
    (`KismetMaterialLibrary.SetScalarParameterValue` "/Game/MP_Pong.MP_Pong" "u_Paddle1Y" (`self.Paddle1Y`) :!label _label)))

(event `InputAction|Paddle1Down`
  (params (Key :type "Key Structure"))
  (:`Pressed`
    (set `self.Paddle1Y` (+ (`self.Paddle1Y`) (`self.PaddleVelocity`)))
    (goto _label)))

(event `InputAction|Paddle2Up`
  (params (Key :type "Key Structure"))
  (:`Pressed`
    (set `self.Paddle2Y` (- (`self.Paddle2Y`) (`self.PaddleVelocity`)))
    (`KismetMaterialLibrary.SetScalarParameterValue` "/Game/MP_Pong.MP_Pong" "u_Paddle2Y" (`self.Paddle2Y`) :!label _label_2)))

(event `InputAction|Paddle2Down`
  (params (Key :type "Key Structure"))
  (:`Pressed`
    (set `self.Paddle2Y` (+ (`self.Paddle2Y`) (`self.PaddleVelocity`)))
    (goto _label_2)))

(fn `UserConstructionScript`
  (`KismetMaterialLibrary.SetScalarParameterValue` "/Game/MP_Pong.MP_Pong" "u_ballRadius" (`self.BallRadius`))
  (`KismetMaterialLibrary.SetScalarParameterValue` "/Game/MP_Pong.MP_Pong" "u_Paddle1Y" (`self.Paddle1Y`))
  (`KismetMaterialLibrary.SetScalarParameterValue` "/Game/MP_Pong.MP_Pong" "u_Paddle2Y" (`self.Paddle2Y`)))